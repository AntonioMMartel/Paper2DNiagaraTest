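; StickArena tracks match statistics for an arena: enemies destroyed and time elapsed.
; An EnemyDestroyed event increments the kill counter each time it is called.
; Tick accumulates delta time into Progress and splits it into whole Minutes and Seconds values.
; BeginPlay and the construction script are empty.
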(event `Enemy Destroyed`
  (set `self.EnemiesDestroyed` (+ (`self.EnemiesDestroyed`) 1)))

(event `self.ReceiveTick`
  (params (DeltaSeconds :type "Float (single-precision)"))
  (bind _output_get (set `self.Progress` (+ DeltaSeconds (`self.Progress`))))
  (set `self.Minutes` (`KismetMathLibrary.FTrunc` (/ _output_get 60.0)))
  (set `self.Seconds` (`KismetMathLibrary.FTrunc` (mod _output_get 60.0))))

(fn `UserConstructionScript`)