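; Paper2D stickman player character that runs along the X axis, jumps and attacks with a mouse-aimed flamethrower through Enhanced Input.
; Tick picks idle, run or falling flipbooks, then sets facing and hand-flame wind from velocity, then from mouse position.
; Attack projects the cursor ray onto the Y=0 plane to orient the Niagara flamethrower while CanFire is true.
; The timed CurrentWeapon.Fire cooldown chain is disconnected.
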(event `self.ReceiveBeginPlay`
  ;[1 1 1] Setup Enhanched Input
  (bind _asstick_player_controller (cast `/Game/Blueprint/Stick_PlayerController` (`self.GetController`)))
  (bind _returnvalue (pcsubsystem `EnhancedInputLocalPlayerSubsystem` _asstick_player_controller))
  (`/Engine/EditorBlueprintResources/StandardMacros.IsValid` _returnvalue
    (:`Is Valid`
      (`EnhancedInputSubsystemInterface.AddMappingContext` _returnvalue "/Game/Blueprint/IMC_PaperPlayer.IMC_PaperPlayer" 0 (struct))
      (set `PlayerController.bShowMouseCursor` true (`GameplayStatics.GetPlayerController` 0)))))

(event `EnhancedInput|/Game/Blueprint/IA_Move`
  (params (ActionValue :type "Float (double-precision)") (ElapsedSeconds :type "Float (double-precision)") (TriggeredSeconds :type "Float (double-precision)") (InputAction :type "InputAction Object Reference" :default "/Game/Blueprint/IA_Move.IA_Move"))
  ;[1 1 1] Execute movement
  (:`Triggered`
    (`self.AddMovementInput` (1.0 0.0 0.0) (* ActionValue (`self.speed`)))))

(event `self.ReceiveTick`
  (params (DeltaSeconds :type "Float (single-precision)"))
  (`self.UpdateAnimations`)
  (`self.UpdateRotation`)
  (`self.UpdateRotationMouse`))

(event `UpdateAnimations`
  (`PaperFlipbookComponent.SetFlipbook` (`self.Sprite`) (select `bool` (`NavMovementComponent.IsFalling` (`self.CharacterMovement`)) :`false` (select `bool` (> (`KismetMathLibrary.VSize` (`MovementComponent.Velocity` (`self.CharacterMovement`))) 0.0) :`false` "/Game/Assets/StickmanPack/Idle/Player_Idle.Player_Idle" :`true` "/Game/Assets/StickmanPack/Run/Player_Run.Player_Run" :!type "PaperFlipbook Object Reference") :`true` "/Game/Assets/StickmanPack/Jump/Player_Falling.Player_Falling")))

(event `EnhancedInput|/Game/Blueprint/IA_Jump`
  (params (ActionValue :type Boolean) (ElapsedSeconds :type "Float (double-precision)") (TriggeredSeconds :type "Float (double-precision)") (InputAction :type "InputAction Object Reference" :default "/Game/Blueprint/IA_Jump.IA_Jump"))
  (:`Started`
    (`self.Jump`))
  (:`Canceled`
    (`self.StopJumping`)))

(event `UpdateRotation`
  (bind _blackflamehandeffect (`self.BlackFlameHandEffect`))
  (`/Engine/EditorBlueprintResources/StandardMacros.IsValid` (`self.GetController`)
    (:`Is Valid`
      (`/Engine/EditorBlueprintResources/StandardMacros.CompareFloat` (.x (`MovementComponent.Velocity` (`self.CharacterMovement`)))
        (:`>`
          (`Controller.SetControlRotation` (`self.GetController`) (`KismetMathLibrary.MakeRotator` 0.0) :!label _label)
          (`NiagaraComponent.SetVariableVec3` _blackflamehandeffect "User.WindDirection" (-1.0 0.0 0.5)))
        (:`<`
          (`Controller.SetControlRotation` (`self.GetController`) (`KismetMathLibrary.MakeRotator` 0.0 0.0 180.0) :!label _label_2)
          (`NiagaraComponent.SetVariableVec3` _blackflamehandeffect "User.WindDirection" (1.0 0.0 0.5)))))))

(event `UpdateRotationMouse`
  (bind _returnvalue (`WidgetLayoutLibrary.GetMousePositionOnViewport`))
  (`/Engine/EditorBlueprintResources/StandardMacros.CompareFloat` (`KismetMathLibrary.BreakVector2D` (`KismetMathLibrary.Conv_VectorToVector2D` (- _returnvalue (`SceneComponent.K2_GetComponentLocation` (`self.Sprite`)))))
    (:`>`
      (goto _label))
    (:`<`
      (goto _label_2))))

(event `EnhancedInput|/Game/Blueprint/IA_Attack`
  (params (ActionValue :type Boolean) (ElapsedSeconds :type "Float (double-precision)") (TriggeredSeconds :type "Float (double-precision)") (InputAction :type "InputAction Object Reference" :default "/Game/Blueprint/IA_Attack.IA_Attack"))
  (bind _returnvalue (`GameplayStatics.GetPlayerController` 0))
  (bind _ng_flamethrowereffect (`self.NG_FlamethrowerEffect`))
  (bind (_locationx _locationy) (`PlayerController.GetMousePosition` _returnvalue))
  (bind (_worldposition _worlddirection) (`GameplayStatics.DeprojectScreenToWorld` _returnvalue (`KismetMathLibrary.Conv_VectorToVector2D` (`KismetMathLibrary.MakeVector` _locationx _locationy))))
  (:`Triggered`
    (if (`self.CanFire`)
      (`NiagaraComponent.SetVariableQuat` _ng_flamethrowereffect "User.Quat" (`KismetMathLibrary.Conv_RotatorToQuaternion` (`KismetMathLibrary.FindLookAtRotation` (`SceneComponent.K2_GetComponentLocation` (`self.Sprite`)) (+ _worldposition (* _worlddirection (`KismetMathLibrary.SafeDivide` (- 0.0 (.y _worldposition)) (.y _worlddirection)))))))
      (`ActorComponent.Activate` _ng_flamethrowereffect false)))
  (:`Canceled`
    (`ActorComponent.Deactivate` (`self.NG_FlamethrowerEffect`) :!label _label_3))
  (:`Completed`
    (goto _label_3)))

(event `EnableFire`
  (set `self.CanFire` true))

(fn `UserConstructionScript`)