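; Enemy projectile actor that flies in a straight line and damages the stickman player on contact.
; Tick moves it along its forward vector by Speed scaled by delta time, without sweeping.
; Overlapping an actor tagged Player calls PlayerDamage with Damage on player character 0, cast to BP_StickmanPlayer.
; The graph never destroys the projectile, neither on hit nor over time.
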(event `self.ReceiveActorBeginOverlap`
  (params (OtherActor :type "Actor Object Reference"))
  (if (`self.ActorHasTag` OtherActor "Player")
    (bind _asbp_stickman_player (cast `/Game/Blueprint/BP_StickmanPlayer` (`GameplayStatics.GetPlayerCharacter` 0)))
    (`/Game/Blueprint/BP_StickmanPlayer.PlayerDamage` _asbp_stickman_player (`self.Damage`))))

(event `self.ReceiveTick`
  (params (DeltaSeconds :type "Float (single-precision)"))
  ;[1 1 1] Update Movement
  (`self.K2_SetActorLocation` (+ (`self.K2_GetActorLocation`) (* (`self.GetActorForwardVector`) (* DeltaSeconds (`self.Speed`))))))

(fn `UserConstructionScript`)